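; Tennis ball actor that reacts to racquet strikes and court bounces to drive rallies and scoring.
; On a hit from a racquet, it takes that racquet's spin, impulse and target to set a new path and records the hitting player's side.
; On court contact it counts bounces, asking the game mode for a bounds check on the first and a points update on the second.
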(event `self.ReceiveHit`
  (params (MyComp :type "PrimitiveComponent Object Reference") (Other :type "Actor Object Reference") (OtherComp :type "PrimitiveComponent Object Reference") (bSelfMoved :type Boolean) (HitLocation :type "Vector Structure") (HitNormal :type "Vector Structure") (NormalImpulse :type "Vector Structure") (Hit :type "HitResult Structure (by ref)"))
  (bind _returnvalue (`GameplayStatics.GetGameMode`))
  (bind _astennis_racquet_bp (cast `/Game/Blueprints/TennisRacquetBP` Other) ; Case Ball struck by Tennis Racquet,\napply new impulse
    (:`then`
      (bind _returnvalue_2 (`TennisRacquet.GetSpin` _astennis_racquet_bp))
      (bind _returnvalue_3 (`TennisRacquet.GetImpulse` _astennis_racquet_bp))
      (bind _returnvalue_4 (`TennisRacquet.GetTarget` _astennis_racquet_bp))
      (`self.SetPath` _returnvalue_2 _returnvalue_3 _returnvalue_4)
      (bind _returnvalue_5 (`TennisRacquet.GetRaqOwner` _astennis_racquet_bp))
      (bind _returnvalue_6 (`TennisPlayer.GetSide` _returnvalue_5))
      (`self.SetLastHit` _returnvalue_6))
    (:`CastFailed`
      (cast `/Game/Blueprints/CourtBP` Other) ; Case Ball bounces against Court,\ncheck for bounds or # of bounces
      (bind _returnvalue_7 (`self.Bounce`))
      (if (== 1 _returnvalue_7)
        (bind _astennis_game_mode_base_bp (cast `/Game/Blueprints/TennisGameModeBaseBP` _returnvalue))
        (`TennisGameModeBase.BoundsCheck` _astennis_game_mode_base_bp (`self.K2_GetActorLocation`))
        (elif (== _returnvalue_7 2)
          (bind _astennis_game_mode_base_bp_2 (cast `/Game/Blueprints/TennisGameModeBaseBP` _returnvalue))
          (`TennisGameModeBase.UpdatePoints` _astennis_game_mode_base_bp_2 0))))))

(fn `UserConstructionScript`)